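; Enemy turret actor that turns to face the first-person player when seen and fires lasers.
; PawnSensing triggers an instant look-at rotation and, after a short Delay that also paces repeated shots, spawns BP_Laser at the LaserSpawner transform.
; Any Hit event decrements EnemyHealth, swapping the mesh material to show damage and destroying the turret at zero.
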(event OnSeePawn(PawnSensing)
  (params (Pawn :type Pawn%20Object%20Reference))
  (bind _asbp_first_person_character (Utilities|Casting|CastToBP_FirstPersonCharacter Pawn))
  (Utilities|FlowControl|Sequence
    (:then_0
      (Transformation|SetActorRotation (Math|Rotator|FindLookatRotation (Transformation|GetActorLocation) (Transformation|GetActorLocation _asbp_first_person_character))))
    (:then_1
      (Utilities|FlowControl|Delay 0.75)
      (Game|SpawnActorfromClass "/Game/Turrets-Enemy_Gunners/BP_Laser.BP_Laser_C" (Transformation|GetWorldTransform (Variables|Default|GetLaserSpawner)) "Undefined" 0 0))))

(event EventBeginPlay)

(event Collision|EventHit
  (params (MyComp :type Primitive%20Component%20Object%20Reference) (Other :type Actor%20Object%20Reference) (OtherComp :type Primitive%20Component%20Object%20Reference) (bSelfMoved :type Boolean) (HitLocation :type Vector :default "0, 0, 0") (HitNormal :type Vector :default "0, 0, 0") (NormalImpulse :type Vector :default "0, 0, 0") (Hit :type Hit%20Result%20Structure%20%28by%20ref%29))
  ;[1 1 1] Health system for the turret. Turret Changes colour to indicate damage done to it
  (bind _output_get (Variables|Default|SetEnemyHealth (- (Variables|Default|GetEnemyHealth) 1)))
  (if (== _output_get 2)
    (Rendering|Material|SetMaterial (Variables|Default|GetStaticMesh) 0 "/Game/FPWeapon/Materials/FirstPersonProjectileMaterial.FirstPersonProjectileMaterial")
    (elif (== (Variables|Default|GetEnemyHealth) 1)
      (Rendering|Material|SetMaterial (Variables|Default|GetStaticMesh) 0 "/Game/FPWeapon/Materials/Enemy.Enemy")
      (elif (== (Variables|Default|GetEnemyHealth) 0)
        (Actor|DestroyActor)))))

(event EventTick
  (params (DeltaSeconds :type Float%20%28single-precision%29)))

(event Collision|EventActorBeginOverlap
  (params (OtherActor :type Actor%20Object%20Reference)))

(fn ConstructionScript)