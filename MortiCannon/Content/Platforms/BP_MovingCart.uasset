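; BP_MovingCart is a cart actor that travels from Position1 through Position2 to Position3 once something overlaps it.
; The first overlap clears the StartTrigger flag, so the move runs only once, and starts a looping timer with no function name set.
; Two chained timelines drive SetActorLocation through vector lerps without sweeping, the second leg starting when the first finishes.
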(event Collision|EventActorBeginOverlap
  (params (OtherActor :type Actor%20Object%20Reference))
  (bind _position2 (Variables|Default|GetPosition2))
  (if (Variables|Default|GetStartTrigger)
    (Variables|Default|SetStartTrigger false)
    (Utilities|Time|SetTimerbyFunctionName 0 "" 1.0 true)
    (bind _new_position (Timeline|LERP%20Timeline Play)
      (:Update
        (Transformation|SetActorLocation self (Math|Vector|Lerp(Vector) (Variables|Default|GetPosition1) _position2 _new_position) false false))
      (:Finished
        (bind _new_position_2 (Timeline|LERP%20Timeline%202 Play)
          (:Update
            (Transformation|SetActorLocation self (Math|Vector|Lerp(Vector) _position2 (Variables|Default|GetPosition3) _new_position_2) false false)))))))

(fn ConstructionScript)