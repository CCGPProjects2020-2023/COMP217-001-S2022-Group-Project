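; BP_Key is an interactable key that opens the door matching its ButtonValue.
; On Interact, it searches every BP_Door in the level for the first one whose DoorValue equals that value.
; It calls OpenDoor on that door with the interacting player, then switches player controller 0's view target to the door and stops searching.
; The view is not switched back in this Blueprint.
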(event EventInteract
  (params (Player :type Character%20Object%20Reference))
  (CallFunction|Key&Door Player))

(fn ConstructionScript)

(fn Key&Door
  (params (Player :type Actor%20Object%20Reference))
  (CallFunction|PerformDoorOpen Player))

(fn PerformDoorOpen
  (params (InputPin :type Actor%20Object%20Reference))
  (bind _outactors (Actor|GetAllActorsOfClass "/Game/Door-Key/BP_Door.BP_Door_C"))
  (bind _array_element (Utilities|Array|ForEachLoopwithBreak _outactors :!label _label)
    (:LoopBody
      (if (== (Variables|/Game/Door-Key/BP_Door.BP_Door_C|GetDoorValue _array_element) (Variables|Default|GetButton%20Value))
        (Default|OpenDoor _array_element InputPin)
        (Game|Player|SetViewTargetwithBlend (Game|GetPlayerController 0) _array_element 0.0 "VTBlend_Linear" 0.0 false)
        (goto _label Break)))))