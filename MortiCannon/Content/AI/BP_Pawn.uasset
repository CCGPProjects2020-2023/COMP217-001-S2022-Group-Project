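; Enemy AI pawn, the gunner, that chases the first-person player and can be destroyed by hits.
; Pawn sensing starts an AI move toward the player and sets CanSeeEnemy, which a retriggerable delay clears shortly after sightings stop.
; Any actor overlap plays a sound and removes one health, swapping the mesh material as health runs low.
; At zero health it plays a death sound, disables collision and destroys itself after a brief delay.
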(event OnSeePawn(PawnSensing)
  (params (Pawn :type Pawn%20Object%20Reference))
  (bind _asbp_first_person_character (Utilities|Casting|CastToBP_FirstPersonCharacter Pawn))
  (Utilities|FlowControl|Sequence
    (:then_0
      (Variables|Default|SetCanSeeEnemy true)
      (AI|AIMoveTo self "0, 0, 0" _asbp_first_person_character 1e+01 false))
    (:then_1
      (Utilities|FlowControl|RetriggerableDelay 0.4)
      (Variables|Default|SetCanSeeEnemy false))))

(event EventBeginPlay)

(event EventTick
  (params (DeltaSeconds :type Float%20%28single-precision%29)))

(event Collision|EventActorBeginOverlap
  (params (OtherActor :type Actor%20Object%20Reference))
  ;[1 1 1] Health system for the gunner. Gunner changes colour depending on remaining health
  (Audio|PlaySound2D "/Game/Audio/bing1.bing1" 0.5 2.0 0.0 0 0)
  (bind _output_get (Variables|Default|SetEnemyHealth (- (Variables|Default|GetEnemyHealth) 1)))
  (if (== _output_get 2)
    (Rendering|Material|SetMaterial (Variables|Character|GetMesh) 0 "/Game/FPWeapon/Materials/FirstPersonProjectileMaterial.FirstPersonProjectileMaterial")
    (elif (== (Variables|Default|GetEnemyHealth) 1)
      (Rendering|Material|SetMaterial (Variables|Character|GetMesh) 0 "/Game/FPWeapon/Materials/Enemy.Enemy")
      (elif (== (Variables|Default|GetEnemyHealth) 0)
        (Rendering|Material|SetMaterial (Variables|Character|GetMesh) 0 "/Game/LevelPrototyping/Materials/M_Solid.M_Solid")
        (Audio|PlaySound2D "/Game/Audio/bell_ding3__2_.bell_ding3__2_" 1.0 1.0 0.0 0 0)
        (Collision|SetActorEnableCollision false)
        (Utilities|FlowControl|Delay 0.25)
        (Actor|DestroyActor)))))

(fn ConstructionScript)